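; BP_EnemyOnPath is an enemy that moves along its own spline path over a set travel time.
; On BeginPlay it detaches the spline keeping world transform, so the path stays put, and scales the timeline's play rate by the inverse of TravelTime.
; Each timeline update samples the spline by time in local space, without constant velocity, and applies the result as the actor location with sweep.
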(event EventBeginPlay
  (|CallParentFunction)
  (Transformation|DetachFromComponent (Variables|Default|GetSpline) "KeepWorld" "KeepWorld" "KeepWorld" true)
  (Components|Timeline|SetPlayRate (Variables|Default|GetTL_MoveAlongSpline) (/ 1.0 (Variables|Default|GetTravelTime)))
  (bind _time (Timeline|TL_MoveAlongSpline PlayFromStart)
    (:Update
      (Transformation|SetActorLocation (Spline|GetLocationatTime (Variables|Default|GetSpline) _time "Local" false) true false))))

(fn ConstructionScript
  (|CallParentFunction))