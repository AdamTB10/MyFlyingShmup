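; BP_Enemy_Turret is an enemy turret that tracks the player and fires bullets on a fixed interval.
; Every tick it turns its Base component in yaw only to face player pawn 0.
; A looping timer started on BeginPlay spawns BP_Enemy_Bullet at the BulletSpawn component's location and rotation, regardless of collision or line of sight.
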(event Custom|ShootBullet
  (bind _bulletspawn (Variables|Default|GetBulletSpawn))
  (bind _returnvalue (Transformation|GetWorldTransform _bulletspawn))
  (Game|SpawnActorfromClass "/Game/Blueprints/Bullets/BP_Enemy_Bullet.BP_Enemy_Bullet_C" (Math|Transform|MakeTransform (.location _returnvalue) (.rotation _returnvalue) "1.000000,1.000000,1.000000") "AlwaysSpawn" "MultiplyWithRoot" 0 0))

(event EventBeginPlay
  (|CallParentFunction)
  (Utilities|Time|SetTimerbyEvent (delegate Custom|ShootBullet) 3.0 true true))

(event Collision|EventActorBeginOverlap
  (params (OtherActor :type Actor%20Object%20Reference))
  (|CallParentFunction OtherActor) ; This node is disabled and will not be called.\nDrag off pins to build functionality.
)

(event EventTick
  (params (DeltaSeconds :type Float%20%28single-precision%29))
  (Transformation|SetWorldRotation (Variables|Default|GetBase) (Math|Rotator|MakeRotator 0.0 0.0 (.yaw (Math|Rotator|FindLookatRotation (Transformation|GetActorLocation) (Transformation|GetActorLocation (Game|Player|GetPlayerPawn 0))))) false false))

(fn ConstructionScript
  (|CallParentFunction))