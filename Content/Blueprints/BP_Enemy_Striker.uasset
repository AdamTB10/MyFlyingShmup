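; BP_Enemy_Striker is an enemy Blueprint that fires repeatedly from its BulletSpawnPoint component.
; On BeginPlay, a looping timer calls ShootBullet every one and a half seconds.
; Each call spawns an actor at the spawn point, waits half a second, then spawns another from the point's current transform, producing two-shot bursts.
; The construction script only calls its parent, and no aiming or movement logic appears here.
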(event Custom|ShootBullet
  (Game|SpawnActorfromClass "/Game/Blueprints/BP_Enemy_Bullet.BP_Enemy_Bullet_C" (Transformation|GetWorldTransform (Variables|Default|GetBulletSpawnPoint)) "Undefined" "MultiplyWithRoot" 0 0)
  (Utilities|FlowControl|Delay 0.5)
  (Game|SpawnActorfromClass "/Game/Blueprints/BP_Enemy_Bullet.BP_Enemy_Bullet_C" (Transformation|GetWorldTransform (Variables|Default|GetBulletSpawnPoint)) "Undefined" "MultiplyWithRoot" 0 0))

(event EventBeginPlay
  (Utilities|Time|SetTimerbyEvent (delegate Custom|ShootBullet) 1.5 true true))

(fn ConstructionScript
  (|CallParentFunction))