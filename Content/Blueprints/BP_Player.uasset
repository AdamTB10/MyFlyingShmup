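; Player ship pawn for a shooter, moved by Enhanced Input and FloatingPawnMovement, banking on strafe.
; Tick aims the turret's yaw at the cursor hit point; fire spawns projectiles by shooting mode (single, two multi-shot patterns, limited bombs), switched by debug keys.
; Overlaps damage the other actor, flash an overlay material and briefly disable collision.
; Damage and pickups update health, relaying HUD, death, lives and bomb changes to the controller.
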(event Custom|UpdatePlayerHealthOnHUD
  ;[0.15 0.15 0.15 0.5] Updating Health UI
  (Class|BPIMyFlyingShmup|SetPlayerHealth(Message) (Pawn|GetController) (/ (Variables|Default|GetHealth) (Variables|Default|GetMaxHealth))))

(event Custom|SetMouseTargetLocation
  (Transformation|SetWorldLocation (Variables|Default|GetMouseTarget) (.Location (Collision|BreakHitResult (.HitResult (Game|Player|GetHitResultUnderCursorbyChannel (Game|GetPlayerController 0) "TraceTypeQuery1" true)))) false false)
  (CallFunction|SetTurretRotation))

(event Custom|SetTurretRotation
  (Transformation|SetWorldRotation (Variables|Default|GetTurretPoint) (Math|Rotator|MakeRotator 0.0 0.0 (.yaw (Math|Rotator|FindLookatRotation (Transformation|GetWorldLocation (Variables|Default|GetTurretPoint)) (Transformation|GetWorldLocation (Variables|Default|GetMouseTarget))))) false false))

(event Custom|InitlisePlayerUI
  ;[0.15 0.15 0.15 0.5] Setting Player Health UI
  (Variables|Default|SetHealth (Variables|Default|GetMaxHealth)))

(event Input|EnhancedActionEvents|EnhancedInputActionIA_MoveForward
  (params (ActionValue :type Boolean) (ElapsedSeconds :type Float%20%28double-precision%29) (TriggeredSeconds :type Float%20%28double-precision%29) (InputAction :type Input%20Action%20Object%20Reference :default "/Game/Inputs/IA_MoveForward.IA_MoveForward"))
  ;[0.15 0.15 0.15 0.5] Movement Inputs
  (Class|PawnMovementComponent|AddInputVector (Variables|Default|GetFloatingPawnMovement) "1.000000,0.000000,0.000000" false))

(event Input|EnhancedActionEvents|EnhancedInputActionIA_MoveBackward
  (params (ActionValue :type Boolean) (ElapsedSeconds :type Float%20%28double-precision%29) (TriggeredSeconds :type Float%20%28double-precision%29) (InputAction :type Input%20Action%20Object%20Reference :default "/Game/Inputs/IA_MoveBackward.IA_MoveBackward"))
  ;[0.15 0.15 0.15 0.5] Movement Inputs
  (Class|PawnMovementComponent|AddInputVector (Variables|Default|GetFloatingPawnMovement) "-1.000000,0.000000,0.000000" false))

(event Input|EnhancedActionEvents|EnhancedInputActionIA_MoveLeft
  (params (ActionValue :type Boolean) (ElapsedSeconds :type Float%20%28double-precision%29) (TriggeredSeconds :type Float%20%28double-precision%29) (InputAction :type Input%20Action%20Object%20Reference :default "/Game/Inputs/IA_MoveLeft.IA_MoveLeft"))
  ;[0.15 0.15 0.15 0.5] Movement Inputs
  (Class|PawnMovementComponent|AddInputVector (Variables|Default|GetFloatingPawnMovement) "0.000000,-1.000000,0.000000" false))

(event Input|EnhancedActionEvents|EnhancedInputActionIA_MoveRight
  (params (ActionValue :type Boolean) (ElapsedSeconds :type Float%20%28double-precision%29) (TriggeredSeconds :type Float%20%28double-precision%29) (InputAction :type Input%20Action%20Object%20Reference :default "/Game/Inputs/IA_MoveRight.IA_MoveRight"))
  ;[0.15 0.15 0.15 0.5] Movement Inputs
  (Class|PawnMovementComponent|AddInputVector (Variables|Default|GetFloatingPawnMovement) "0.000000,1.000000,0.000000" false))

(event Input|EnhancedActionEvents|EnhancedInputActionIA_PrimaryFire
  (params (ActionValue :type Boolean) (ElapsedSeconds :type Float%20%28double-precision%29) (TriggeredSeconds :type Float%20%28double-precision%29) (InputAction :type Input%20Action%20Object%20Reference :default "/Game/Inputs/IA_PrimaryFire.IA_PrimaryFire"))
  (bind _projectilespawnpoint (Variables|Default|GetProjectileSpawnPoint))
  (bind _projectilespawnpoint_2 (Variables|Default|GetProjectileSpawnPoint))
  (bind _returnvalue (Transformation|GetWorldTransform _projectilespawnpoint_2))
  (bind _returnvalue_2 (Transformation|GetWorldTransform _projectilespawnpoint))
  ;[0.15 0.15 0.15 0.5] Primary Fire
  (switch int (Variables|Default|GetShootingModeIndex)
    (:0
      ;[0.15 0.15 0.15 0.5] Shooting Mode 0
      (Utilities|FlowControl|Delay 0.3)
      (Game|SpawnActorfromClass "/Game/Blueprints/Bullets/BP_Player_Bullet.BP_Player_Bullet_C" (Transformation|GetWorldTransform (Variables|Default|GetProjectileSpawnPoint)) "AlwaysSpawn" "MultiplyWithRoot" 0 0)
      (Audio|PlaySound2D "/Game/Sci-Fi_Shots_Pack2_Game_Of_Weapons/Cue/SciFi_Shot_P2__126__Cue.SciFi_Shot_P2__126__Cue" 1.0 1.0 0.0 0 0))
    (:1
      ;[0.15 0.15 0.15 0.5] Shooting Mode 1
      (Utilities|FlowControl|Delay 0.3)
      (for _array_element (Variables|Default|GetShootingMode1Transforms)
        (Game|SpawnActorfromClass "/Game/Blueprints/Bullets/BP_Player_Bullet_Multi.BP_Player_Bullet_Multi_C" (Math|Transform|MakeTransform (.location _returnvalue_2) (Math|Rotator|CombineRotators (Math|Rotator|MakeRotator (.roll _array_element) (.pitch _array_element) (.yaw _array_element)) (Math|Rotator|MakeRotator 0.0 0.0 (.yaw (.rotation _returnvalue_2)))) "1.000000,1.000000,1.000000") "AlwaysSpawn" "MultiplyWithRoot" 0 0)
        (Audio|PlaySound2D "/Game/Sci-Fi_Shots_Pack2_Game_Of_Weapons/Cue/SciFi_Shot_P2__50__Cue.SciFi_Shot_P2__50__Cue" 0.25 1.0 0.0 0 0)))
    (:2
      ;[0.15 0.15 0.15 0.5] Shooting Mode 2
      (Utilities|FlowControl|Delay 0.3)
      (for _array_element_2 (Variables|Default|GetShootingMode2Transforms)
        (Game|SpawnActorfromClass "/Game/Blueprints/Bullets/BP_Player_Bullet_Multi.BP_Player_Bullet_Multi_C" (Math|Transform|MakeTransform (+ (.location _array_element_2) (.location _returnvalue)) (Math|Rotator|CombineRotators (.rotation _array_element_2) (.rotation _returnvalue)) "1.000000,1.000000,1.000000") "AlwaysSpawn" "MultiplyWithRoot" 0 0)
        (Audio|PlaySound2D "/Game/Sci-Fi_Shots_Pack2_Game_Of_Weapons/Cue/SciFi_Shot_P2__50__Cue.SciFi_Shot_P2__50__Cue" 0.25 1.0 0.0 0 0)))
    (:3
      ;[0.15 0.15 0.15 0.5] Shooting Mode 3
      (bind _asmy_player_controller (Utilities|Casting|CastTomyPlayerController (Pawn|GetController)))
      (if (> (Variables|/Game/Framework/myPlayerController.myPlayerController_C|GetCurrentBombCount _asmy_player_controller) 0)
        (Utilities|FlowControl|Delay 0.3)
        (Game|SpawnActorfromClass "/Game/Blueprints/Bullets/BP_Player_Bomb.BP_Player_Bomb_C" (Transformation|GetWorldTransform (Variables|Default|GetProjectileSpawnPoint)) "AlwaysSpawn" "MultiplyWithRoot" 0 0)
        (Audio|PlaySound2D "/Game/Sci-Fi_Shots_Pack2_Game_Of_Weapons/Cue/SciFi_Shot_P2__116__Cue.SciFi_Shot_P2__116__Cue" 1.0 1.0 0.0 0 0)
        (Class|BPIMyFlyingShmup|SetPlayerBombCount(Message) (Pawn|GetController) -1)))))

(event EventBeginPlay
  ;[0.15 0.15 0.15 0.5] Mapping Context
  (bind _asplayer_controller (Utilities|Casting|CastToPlayerController (Pawn|GetController)))
  (Input|AddMappingContext (PlayerController|LocalPlayerSubsystems|GetEnhancedInputLocalPlayerSubsystem _asplayer_controller) "/Game/Inputs/IMC_myFirstPlayerPawn.IMC_myFirstPlayerPawn" 0 "(bIgnoreAllPressedKeysUntilRelease=True,bForceImmediately=False,bNotifyUserSettings=False)")
  ;[0.15 0.15 0.15 0.5] Rotate Propeller
  (Components|Movement|SetUpdatedComponent (Variables|Default|GetEngineBoosterRotation) (Variables|Default|GetEngineBooster))
  (CallFunction|InitlisePlayerUI))

(event Collision|EventActorBeginOverlap
  (params (OtherActor :type Actor%20Object%20Reference))
  (Game|Damage|ApplyDamage OtherActor (Variables|Default|GetMaxHealth) 0 0)
  (Audio|PlaySound2D "/Game/Sci-Fi_Shots_Pack2_Game_Of_Weapons/Cue/SciFi_Shot_P2__176__Cue.SciFi_Shot_P2__176__Cue" 1.0 1.0 0.0 0 0)
  (Rendering|Material|SetOverlayMaterial (Variables|Default|GetShip) "/Game/Materials/Damage/MI_Damage_Flash.MI_Damage_Flash" :!class /Script/Engine.MeshComponent)
  (Collision|SetActorEnableCollision false)
  (Utilities|FlowControl|Delay 0.3)
  (Rendering|Material|SetOverlayMaterial (Variables|Default|GetShip) 0 :!class /Script/Engine.MeshComponent)
  (Utilities|FlowControl|Delay 0.6)
  (Collision|SetActorEnableCollision true))

(event Game|Damage|EventAnyDamage
  (params (Damage :type Float%20%28single-precision%29) (DamageType :type Damage%20Type%20Object%20Reference) (InstigatedBy :type Controller%20Object%20Reference) (DamageCauser :type Actor%20Object%20Reference))
  ;[0.15 0.15 0.15 0.5] Health System
  (bind _output_get (Variables|Default|SetHealth (Math|Float|Clamp(Float) (- (Variables|Default|GetHealth) Damage) 0.0 (Variables|Default|GetMaxHealth))))
  (CallFunction|UpdatePlayerHealthonHUD)
  (if (== _output_get 0.0)
    (Collision|SetActorEnableCollision false)
    (Class|BPIMyFlyingShmup|OnPlayerDeath(Message) (Pawn|GetController))))

(event EventTick
  (params (DeltaSeconds :type Float%20%28single-precision%29))
  ;[0.15 0.15 0.15 0.5] Banking Mechanic
  (CallFunction|SetMouseTargetLocation)
  (bind _output_get (Variables|Default|SetTagetBank%20Angle (Math|Float|SelectFloat -1.0 (Math|Float|SelectFloat 1.0 0.0 (Input|EnhancedActionValues|GetIA_MoveRight)) (Input|EnhancedActionValues|GetIA_MoveLeft))))
  (Variables|Default|SetCurrentBankAngle (Math|Interpolation|FInterpTo (Variables|Default|GetCurrentBankAngle) _output_get DeltaSeconds 6.0))
  (Transformation|SetRelativeRotation (Variables|Default|GetBox) (Math|Rotator|MakeRotator (* (Variables|Default|GetMaxBankAngle) (Variables|Default|GetCurrentBankAngle)) 0.0 0.0) false false))

(event EventOnPickup
  (params (HealthToAdd :type Float%20%28double-precision%29) (ShouldIncreaseMaxHealth :type Boolean) (PlayerLivesToAdd :type Integer) (BombsToAdd :type Integer))
  (Utilities|FlowControl|Sequence
    (:then_0
      (Variables|Default|SetHealth (+ HealthToAdd (Variables|Default|GetHealth))))
    (:then_1
      (if ShouldIncreaseMaxHealth
        (Variables|Default|SetMaxHealth (+ HealthToAdd (Variables|Default|GetMaxHealth)))))
    (:then_2
      (CallFunction|UpdatePlayerHealthonHUD))
    (:then_3
      (Class|BPIMyFlyingShmup|ModifyPlayerLives(Message) (Pawn|GetController) PlayerLivesToAdd))
    (:then_4
      (Class|BPIMyFlyingShmup|SetPlayerBombCount(Message) (Pawn|GetController) BombsToAdd))))

(event Input|KeyboardEvents|DebugKeyM
  (params (Key :type Key%20Structure :default "None") (ActionValue :type Input%20Action%20Value%20Structure))
  ;[0.15 0.15 0.15 0.5] Modify Shooting Mode
  (:Pressed
    (Math|Integer|IncrementInt (Variables|Default|GetShootingModeIndex))))

(event Input|KeyboardEvents|DebugKeyN
  (params (Key :type Key%20Structure :default "None") (ActionValue :type Input%20Action%20Value%20Structure))
  ;[0.15 0.15 0.15 0.5] Modify Shooting Mode
  (:Pressed
    (Math|Integer|DecrementInt (Variables|Default|GetShootingModeIndex))))

(fn ConstructionScript)